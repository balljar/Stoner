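; BP_Portal_3 is the end-of-level portal for Level 3.
; On overlap it locks the third-person character, stops its capsule physics and uses a timeline to pull it toward the portal center.
; On reaching the center, it saves a faster time to the SoundGameInstance arrays and shows the Level_End widget with UI-only input.
; Tick polls that widget's flags to open Level4 or replay Level3.
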(event `self.ReceiveTick`
  (params (DeltaSeconds :type "Float (single-precision)"))
  (bind _reference_to_level_end_widget (`self.Reference To Level End Widget`))
  ;[1 1 1] Widget Button functionality
  (`/Engine/EditorBlueprintResources/StandardMacros.IsValid` _reference_to_level_end_widget
    (:`Is Valid`
      (if (`/Game/Blueprint/Portals/Level_End.NextLevel` _reference_to_level_end_widget)
        (`GameplayStatics.OpenLevelBySoftObjectPtr` "/Game/ThirdPerson/Maps/Levels/Level4.Level4")
        (elif (`/Game/Blueprint/Portals/Level_End.ReplayLevel` _reference_to_level_end_widget)
          (`GameplayStatics.OpenLevelBySoftObjectPtr` "/Game/ThirdPerson/Maps/Levels/Level3.Level3"))))))

(event `self.ReceiveActorBeginOverlap`
  (params (OtherActor :type "Actor Object Reference"))
  (bind _returnvalue (`GameplayStatics.GetPlayerController` 0))
  (bind _asbp_third_person_character (cast `/Game/ThirdPerson/Blueprints/BP_ThirdPersonCharacter` OtherActor))
  (set `/Game/ThirdPerson/Blueprints/BP_ThirdPersonCharacter.CanMove` false _asbp_third_person_character)
  (set `/Game/ThirdPerson/Blueprints/BP_ThirdPersonCharacter.InPortal?` true _asbp_third_person_character)
  (bind _capsulecomponent (`Character.CapsuleComponent` _asbp_third_person_character))
  (`PrimitiveComponent.SetAngularDamping` _capsulecomponent 100.0)
  (`PrimitiveComponent.SetEnableGravity` _capsulecomponent false)
  (`PrimitiveComponent.SetSimulatePhysics` _capsulecomponent false)
  (bind (_direction _newtrack_0) (`Timeline|Movement Timeline`)
    (:`Update`
      (`SceneComponent.K2_SetWorldLocation` _capsulecomponent (`KismetMathLibrary.VLerp` (`SceneComponent.K2_GetComponentLocation` _capsulecomponent) (`SceneComponent.K2_GetComponentLocation` (`self.Portal Center`)) _newtrack_0) false false)
      (if (`PrimitiveComponent.IsOverlappingComponent` _capsulecomponent (`self.Portal Center`))
        (set `self.InPortal` true)
        (`KismetSystemLibrary.Delay` 1.0)
        (bind _assound_game_instance (cast `/Game/Blueprint/SoundGameInstance` (`GameplayStatics.GetGameInstance`)))
        (bind _minutes (`/Game/ThirdPerson/Blueprints/BP_ThirdPersonCharacter.Minutes` _asbp_third_person_character))
        (bind _seconds (`/Game/ThirdPerson/Blueprints/BP_ThirdPersonCharacter.Seconds` _asbp_third_person_character))
        ;[1 1 1] SetFastestTime
        (if (< (+ (* _minutes 60) _seconds) (+ (* (`|GetArrayItem` (`/Game/Blueprint/SoundGameInstance.MWorld1` _assound_game_instance) 2) 60) (`|GetArrayItem` (`/Game/Blueprint/SoundGameInstance.SWorld1` _assound_game_instance) 2)))
          (`KismetArrayLibrary.Array_Set` (`/Game/Blueprint/SoundGameInstance.MWorld1` _assound_game_instance) 2 _minutes)
          (`KismetArrayLibrary.Array_Set` (`/Game/Blueprint/SoundGameInstance.SWorld1` _assound_game_instance) 2 _seconds))
        (bind _returnvalue_2 (`|CreateWidget` "/Game/Blueprint/Portals/Level_End.Level_End_C" _returnvalue))
        (bind _output_get (set `self.Reference To Level End Widget` _returnvalue_2))
        (`UserWidget.AddToViewport` _returnvalue_2 0)
        (`UserWidget.AddToViewport` _output_get 0)
        (`WidgetBlueprintLibrary.SetInputMode_UIOnlyEx` _returnvalue _output_get)
        (set `PlayerController.bShowMouseCursor` true _returnvalue)
        (else
          (set `self.InPortal` false))))))

(fn `UserConstructionScript`)