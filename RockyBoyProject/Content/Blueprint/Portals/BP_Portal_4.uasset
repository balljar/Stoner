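; BP_Portal_4 is a level-exit portal that pulls the player character in and loads Level5.
; On overlap it disables the character's movement, raises capsule angular damping and plays a timeline that lerps the capsule toward PortalCenter.
; Once the capsule overlaps PortalCenter, it sets InPortal, waits briefly, destroys the character and opens the level.
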(event `self.ReceiveActorBeginOverlap`
  (params (OtherActor :type "Actor Object Reference"))
  (bind _asbp_third_person_character (cast `/Game/ThirdPerson/Blueprints/BP_ThirdPersonCharacter` OtherActor))
  (set `/Game/ThirdPerson/Blueprints/BP_ThirdPersonCharacter.CanMove` false _asbp_third_person_character)
  (bind _capsulecomponent (`Character.CapsuleComponent` _asbp_third_person_character))
  (`PrimitiveComponent.SetAngularDamping` _capsulecomponent 100.0)
  (bind (_direction _newtrack_0) (`Timeline|Movement Timeline`)
    (:`Update`
      (`SceneComponent.K2_SetWorldLocation` _capsulecomponent (`KismetMathLibrary.VLerp` (`SceneComponent.K2_GetComponentLocation` _capsulecomponent) (`SceneComponent.K2_GetComponentLocation` (`self.Portal Center`)) _newtrack_0) false false)
      (if (`PrimitiveComponent.IsOverlappingComponent` _capsulecomponent (`self.Portal Center`))
        (set `self.InPortal` true)
        (`KismetSystemLibrary.Delay` 1.0)
        (`self.K2_DestroyActor` _asbp_third_person_character)
        (`GameplayStatics.OpenLevelBySoftObjectPtr` "/Game/ThirdPerson/Maps/Levels/Level5.Level5")
        (else
          (set `self.InPortal` false))))))

(fn `UserConstructionScript`)