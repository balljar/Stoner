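; Jump pad actor that launches any Character entering its Box trigger along the forward direction of its Arrow component.
; On overlap, a velocity-change impulse on the capsule first cancels vertical velocity and adjusts horizontal velocity by a VelocityDamp factor.
; A second impulse, scaled by Strength, then applies the launch, and a 2D jump sound plays.
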(event `self.Box.OnComponentBeginOverlap`
  (params (OverlappedComponent :type "PrimitiveComponent Object Reference") (OtherActor :type "Actor Object Reference") (OtherComp :type "PrimitiveComponent Object Reference") (OtherBodyIndex :type Integer) (bFromSweep :type Boolean) (SweepResult :type "HitResult Structure (by ref)"))
  (bind _velocitydamp (`self.VelocityDamp`))
  (bind _ascharacter (cast `Character` OtherActor))
  (bind _capsulecomponent (`Character.CapsuleComponent` _ascharacter))
  (bind (_returnvalue_x _returnvalue_y _returnvalue_z) (`KismetMathLibrary.BreakVector` (`self.GetVelocity` _ascharacter)))
  (`PrimitiveComponent.AddImpulse` _capsulecomponent (`KismetMathLibrary.MakeVector` (* _returnvalue_x _velocitydamp) (* _returnvalue_y _velocitydamp) (* _returnvalue_z -1.0)) "None" true)
  (`PrimitiveComponent.AddImpulse` _capsulecomponent (* (`SceneComponent.GetForwardVector` (`self.Arrow`)) (`self.Strength`)) "None" true)
  (`GameplayStatics.PlaySound2D` "/Game/SoundEffects/new_jump.new_jump" 1.0 1.0 0.0 null null))

(fn `UserConstructionScript`)