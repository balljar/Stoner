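; CheckPoint1 is a checkpoint trigger actor that logs a timer split for the player, apparently for "W2".
; When BP_ThirdPersonCharacter enters its Box, it overwrites SoundGameInstance's W2CheckPoints array so only index 1 is true, making the following check always pass.
; It then prints a debug string, stores the character's Minutes (not Seconds) in W2Record index 1 and resets both timer values.
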(event `self.Box.OnComponentBeginOverlap`
  (params (OverlappedComponent :type "PrimitiveComponent Object Reference") (OtherActor :type "Actor Object Reference") (OtherComp :type "PrimitiveComponent Object Reference") (OtherBodyIndex :type Integer) (bFromSweep :type Boolean) (SweepResult :type "HitResult Structure (by ref)"))
  (bind _asbp_third_person_character (cast `/Game/ThirdPerson/Blueprints/BP_ThirdPersonCharacter` OtherActor))
  (bind _assound_game_instance (cast `/Game/Blueprint/SoundGameInstance` (`GameplayStatics.GetGameInstance`)))
  (set `/Game/Blueprint/SoundGameInstance.W2CheckPoints` (`|MakeArray` false true false false) _assound_game_instance)
  (if (`|GetArrayItem` (`/Game/Blueprint/SoundGameInstance.W2CheckPoints` _assound_game_instance) 1)
    (`KismetSystemLibrary.PrintString` "Check1")
    (`KismetArrayLibrary.Array_Set` (`/Game/Blueprint/SoundGameInstance.W2Record` _assound_game_instance) 1 (`/Game/ThirdPerson/Blueprints/BP_ThirdPersonCharacter.Minutes` _asbp_third_person_character))
    (set `/Game/ThirdPerson/Blueprints/BP_ThirdPersonCharacter.Minutes` 0 _asbp_third_person_character)
    (set `/Game/ThirdPerson/Blueprints/BP_ThirdPersonCharacter.Seconds` 0 _asbp_third_person_character)))

(fn `UserConstructionScript`)