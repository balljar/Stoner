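; Gravity well actor that pulls the third-person character toward the center of its Sphere1 component.
; On sphere overlap it stores the character, sets InRange and applies a fixed sideways launch impulse.
; While InRange, which nothing here clears, Tick disables the capsule's gravity and applies a velocity-change impulse toward the center.
; GravForce adds an inverse-distance term to Strength for that pull and prints the capsule's speed.
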(event `self.ReceiveTick`
  (params (DeltaSeconds :type "Float (single-precision)"))
  (if (`self.InRange`)
    (bind _capsulecomponent (`Character.CapsuleComponent` (stale `self.Sphere1.OnComponentBeginOverlap` _asbp_third_person_character)))
    (`PrimitiveComponent.SetEnableGravity` _capsulecomponent false)
    (`self.Grav Force` (stale `self.Sphere1.OnComponentBeginOverlap` _asbp_third_person_character))
    (else
      (`PrimitiveComponent.SetEnableGravity` _capsulecomponent true))))

(event `self.Sphere1.OnComponentBeginOverlap`
  (params (OverlappedComponent :type "PrimitiveComponent Object Reference") (OtherActor :type "Actor Object Reference") (OtherComp :type "PrimitiveComponent Object Reference") (OtherBodyIndex :type Integer) (bFromSweep :type Boolean) (SweepResult :type "HitResult Structure (by ref)"))
  (bind _asbp_third_person_character (cast `/Game/ThirdPerson/Blueprints/BP_ThirdPersonCharacter` OtherActor))
  (set `self.InRange` true)
  (`PrimitiveComponent.AddImpulse` (`Character.CapsuleComponent` _asbp_third_person_character) (-5000.0 5000.0 0.0) "None" true))

(fn `Grav Force`
  (params (Capsule :type "Character Object Reference"))
  (bind _capsulecomponent (`Character.CapsuleComponent` Capsule))
  (bind _returnvalue (`SceneComponent.K2_GetComponentLocation` (`self.Sphere1`)))
  (bind _returnvalue_2 (`SceneComponent.K2_GetComponentLocation` _capsulecomponent))
  (`PrimitiveComponent.AddImpulse` _capsulecomponent (* (`KismetMathLibrary.GetDirectionUnitVector` _returnvalue_2 _returnvalue) (+ (`self.Strength`) (/ 100000.0 (`KismetMathLibrary.Vector_Distance` _returnvalue _returnvalue_2)))) "None" true)
  (`KismetSystemLibrary.PrintString` (`KismetStringLibrary.Conv_DoubleToString` (`KismetMathLibrary.VSize` (`SceneComponent.GetComponentVelocity` _capsulecomponent)))))

(fn `UserConstructionScript`)